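; BP_SubGoalJournal displays quest sub-goals in a journal widget hosted by its Widget component.
; On BeginPlay it casts that widget to w_SubGoalJournal, then creates one W_SubGoals entry per sub-goal across the Quests array and adds it to the SubGoals container.
; The list is built only once, with Russian debug prints tracing the loops and a failed cast, while the FillJournal event is an empty stub.
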(event `self.ReceiveBeginPlay`
  (bind _quests (`self.Quests`))
  (bind _asw_sub_goal_journal (cast `/Game/Widgets/w_SubGoalJournal` (`WidgetComponent.GetUserWidgetObject` (`self.Widget`)))
    (:`then`
      (`KismetSystemLibrary.PrintString` (`KismetStringLibrary.Concat_StrStr` "длина в виджете" (`KismetStringLibrary.Conv_IntToString` (`KismetArrayLibrary.Array_Length` _quests))) true true (struct :`R` 1.0 :`B` 0.059353 :`A` 1.0) 15.0)
      (for _array_element _quests
        (`KismetSystemLibrary.PrintString` "квест")
        (for _array_element_2 (`.SubGoals_40_5961F38549EB76530A0BA0843BB03DF9` (break `/Game/Structures/s_QuestInfo` (`/Game/Blueprints/Quests/BP_MasterQuest.QuestInfo` _array_element)))
          (bind _returnvalue (`|CreateWidget` "/Game/Widgets/w_SubGoals.w_SubGoals_C" (`GameplayStatics.GetPlayerController` 0) _array_element_2))
          (`PanelWidget.AddChild` (`/Game/Widgets/w_SubGoalJournal.SubGoals` _asw_sub_goal_journal) _returnvalue)
          (`KismetSystemLibrary.PrintString` "подзадача"))))
    (:`CastFailed`
      (`KismetSystemLibrary.PrintString` "не кастит"))))

(event `FillJournal`)

(fn `UserConstructionScript`)