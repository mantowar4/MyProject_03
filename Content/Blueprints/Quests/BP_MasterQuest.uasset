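; BP_MasterQuest is a quest actor that tracks a quest's subgoals and shows them in the main widget's quest list.
; SetupStartingGoals activates every subgoal in QuestInfo, creating a W_SubGoals entry for each.
; CompleteSubGoals removes an active goal by index, rebuilds the current goal list and detaches its widget.
; When no goals remain, it sets quest success on BP_GameInstance, clears FirstQuest and opens the "room" level.
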(fn `AddGoalForIndex`
  (params (Index :type Integer))
  (locals (LocalIndex :type Integer))
  (bind _mainwidget (`self.MainWidget`))
  (bind _goal (`self.GoalAtIndex` (`local.LocalIndex`)))
  (bind _output_get (set `local.LocalIndex` Index))
  (if (`self.GoalFound?` _output_get)
    (`KismetArrayLibrary.Array_Add` (`self.CurrentGoalIndicies`) (`local.LocalIndex`))
    (`KismetArrayLibrary.Array_Add` (`self.CurrentGoal`) _goal)
    (bind _returnvalue (`|CreateWidget` "/Game/Widgets/w_SubGoals.w_SubGoals_C" null _goal))
    (`PanelWidget.AddChild` (`/Game/Widgets/w_MainWidget.QuestList` _mainwidget) _returnvalue)
    (`KismetArrayLibrary.Array_Add` (`/Game/Widgets/w_MainWidget.SubGoals` _mainwidget) _returnvalue)
    (return)))

(fn `CompleteSubGoals`
  (params (SubGoalIndex :type Integer))
  (returns (`Success?` :type Boolean))
  (locals (LocalGoalIndex :type Integer) (LocalCompletedGoal :type "/Game/Structures/s_GoalInfo Structure") (LocalWidgetIndex :type Integer))
  (bind _localwidgetindex (`local.LocalWidgetIndex`))
  (bind (_name _description _subgoals) (break `/Game/Structures/s_QuestInfo` (`self.QuestInfo`)))
  (set `local.LocalGoalIndex` SubGoalIndex)
  (if (`KismetArrayLibrary.Array_Contains` (`self.CurrentGoalIndicies`) (`local.LocalGoalIndex`))
    (bind _output_get (set `local.LocalCompletedGoal` (`|GetArrayItem` _subgoals (`local.LocalGoalIndex`))))
    (`KismetArrayLibrary.Array_RemoveItem` (`self.CurrentGoal`) (`local.LocalCompletedGoal`))
    (set `local.LocalWidgetIndex` (`KismetArrayLibrary.Array_Find` _subgoals _output_get))
    (`KismetArrayLibrary.Array_RemoveItem` (`self.CurrentGoalIndicies`) (`local.LocalGoalIndex`))
    (`self.UpdateSubGoals`)
    (`KismetSystemLibrary.PrintString` (`KismetStringLibrary.Concat_StrStr` "WidgetIndex : " (`KismetStringLibrary.Conv_IntToString` _localwidgetindex)))
    (`Widget.RemoveFromParent` (`|GetArrayItem` (`/Game/Widgets/w_MainWidget.SubGoals` (`self.MainWidget`)) _localwidgetindex))
    (if (<= (`KismetArrayLibrary.Array_Length` (`self.CurrentGoal`)) 0)
      (bind _asbp_game_instance (cast `/Game/Blueprints/BP_GameInstance` (`GameplayStatics.GetGameInstance`)))
      (set `/Game/Blueprints/BP_GameInstance.FirstQuest?` false _asbp_game_instance)
      (set `/Game/Blueprints/BP_GameInstance.QuestSuccess?` true _asbp_game_instance)
      (`GameplayStatics.OpenLevel` "room"))
    (else
      (return false))))

(fn `GoalAtIndex`
  (params (Index :type Integer))
  (returns (Goal :type "/Game/Structures/s_GoalInfo Structure"))
  (return (`|GetArrayItem` (`.SubGoals_40_5961F38549EB76530A0BA0843BB03DF9` (break `/Game/Structures/s_QuestInfo` (`self.QuestInfo`))) Index)))

(fn `GoalFound?`
  (params (Index :type Integer))
  (returns (Out :type Boolean))
  (return (< Index (`KismetArrayLibrary.Array_Length` (`.SubGoals_40_5961F38549EB76530A0BA0843BB03DF9` (break `/Game/Structures/s_QuestInfo` (`self.QuestInfo`)))))))

(fn `SetupStartingGoals`
  (`KismetArrayLibrary.Array_Clear` (`self.CurrentGoalIndicies`))
  (for (_ _array_index) (`.SubGoals_40_5961F38549EB76530A0BA0843BB03DF9` (break `/Game/Structures/s_QuestInfo` (`self.QuestInfo`)))
    (`KismetArrayLibrary.Array_Add` (`self.StartingSubGoalIndices`) _array_index))
  (for _array_element (`self.StartingSubGoalIndices`)
    (`self.AddGoalForIndex` _array_element)))

(fn `UpdateSubGoals`
  (`KismetArrayLibrary.Array_Clear` (`self.CurrentGoal`))
  (for _array_element (`self.CurrentGoalIndicies`)
    (`KismetArrayLibrary.Array_Add` (`self.CurrentGoal`) (`|GetArrayItem` (`.SubGoals_40_5961F38549EB76530A0BA0843BB03DF9` (break `/Game/Structures/s_QuestInfo` (`self.QuestInfo`))) _array_element)))
  (return))

(fn `UserConstructionScript`)