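; Quest manager for a VR game that tracks active quests as spawned actors and records every quest class given.
; AddNewQuest ignores repeats, spawns the quest, starts its goals and places a sub-goal journal actor facing the player.
; AddQuestToList adds a journal widget to the main UI, always titled with the first quest's name.
; OnInteractGoal waits briefly, then completes current sub-goals whose class matches the interacted goal.
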(event `OnInteractGoal`
  (params (InteractGoal :type "/Game/Blueprints/GoalsInteract/BP_GoalsInteractMaster Class Reference"))
  (`KismetSystemLibrary.Delay` 5.0)
  (`KismetArrayLibrary.Array_Clear` (`self.IndicesToCompleteLater`))
  (set `self.InteractGoal` InteractGoal)
  (for _array_element (`self.CurrentQuestActors`)
    (for (_array_element_2 _array_index) (`/Game/Blueprints/Quests/BP_MasterQuest.CurrentGoal` _array_element)
      (if (== (`.GoalClass_49_9BD7E5204BC4BF7AB30C96BD64E67857` (break `/Game/Structures/s_GoalInfo` _array_element_2)) (`self.InteractGoal`))
        (`/Game/Blueprints/Quests/BP_MasterQuest.CompleteSubGoals` _array_element (`|GetArrayItem` (`/Game/Blueprints/Quests/BP_MasterQuest.CurrentGoalIndicies` _array_element) _array_index))))))

(fn `AddNewQuest`
  (params (NewQuest :type "/Game/Blueprints/Quests/BP_MasterQuest Class Reference"))
  (locals (L_QuestClass :type "/Game/Blueprints/Quests/BP_MasterQuest Class Reference") (L_QuestActor :type "/Game/Blueprints/Quests/BP_MasterQuest Object Reference"))
  (bind _vrpawn (`self.VRPawn`))
  (bind _currentquestactors (`self.CurrentQuestActors`))
  (bind _l_questactor (`local.L_QuestActor`))
  (bind _returnvalue (`self.K2_GetActorLocation` _vrpawn))
  (set `local.L_QuestClass` NewQuest)
  (if (and (`KismetSystemLibrary.IsValidClass` NewQuest) (not (`KismetArrayLibrary.Array_Contains` (`self.AllQuestClasses`) NewQuest)))
    (`KismetArrayLibrary.Array_Add` (`self.AllQuestClasses`) (`local.L_QuestClass`))
    (bind _returnvalue_2 (`|SpawnActorFromClass` (`local.L_QuestClass`) (`KismetMathLibrary.MakeTransform` (0.0 0.0 0.0)) "Undefined" "OverrideRootScale" null null))
    (set `local.L_QuestActor` _returnvalue_2)
    (`KismetArrayLibrary.Array_Add` _currentquestactors _l_questactor)
    (for _array_element _currentquestactors
      (`KismetSystemLibrary.PrintString` (`KismetTextLibrary.Conv_TextToString` (`.Name_2_9CFE47C748EDE7F5A3B8EF84947AAD28` (break `/Game/Structures/s_QuestInfo` (`/Game/Blueprints/Quests/BP_MasterQuest.QuestInfo` _array_element))))))
    (`self.AddQuestToList` _l_questactor)
    (set `/Game/Blueprints/Quests/BP_MasterQuest.MainWidget` (`self.MainWidgetRef`) _l_questactor)
    (`/Game/Blueprints/Quests/BP_MasterQuest.SetupStartingGoals` _l_questactor)
    (bind _returnvalue_3 (`|SpawnActorFromClass` "/Game/Blueprints/BP_SubGoalJournal.BP_SubGoalJournal_C" (`KismetMathLibrary.MakeTransform` (+ _returnvalue (* (`KismetMathLibrary.GetForwardVector` (`SceneComponent.K2_GetComponentRotation` (`/Game/VirtualRealityBP/Blueprints/MotionControllerPawn.CapsuleCollision` _vrpawn))) 200.0))) "Undefined" "OverrideRootScale" _vrpawn (`self.CurrentQuestActors`) null))
    (`self.K2_SetActorRotation` _returnvalue_3 (`KismetMathLibrary.FindLookAtRotation` (`self.K2_GetActorLocation` _returnvalue_3) _returnvalue) false)
    (else
      (return))))

(fn `AddQuestToList`
  (params (Quest :type "/Game/Blueprints/Quests/BP_MasterQuest Object Reference"))
  (`/Engine/EditorBlueprintResources/StandardMacros.IsValid` Quest
    (:`Is Valid`
      (bind _returnvalue (`|CreateWidget` "/Game/Widgets/w_QuestJournal.w_QuestJournal_C" (`GameplayStatics.GetPlayerController` 0)))
      (`TextBlock.SetText` (`/Game/Widgets/w_QuestJournal.QuestHead` _returnvalue) (`.Name_2_9CFE47C748EDE7F5A3B8EF84947AAD28` (break `/Game/Structures/s_QuestInfo` (`/Game/Blueprints/Quests/BP_MasterQuest.QuestInfo` (`|GetArrayItem` (`self.CurrentQuestActors`))))))
      (`PanelWidget.AddChild` (`/Game/Widgets/w_MainWidget.QuestList` (`self.MainWidgetRef`)) _returnvalue))
    (:`Is Not Valid`
      (return))))

(fn `HasCurrentQuest?`
  (params (QuestClass :type "/Game/Blueprints/Quests/BP_MasterQuest Class Reference"))
  (returns (`Out?` :type Boolean) (QuestActor :type "/Game/Blueprints/Quests/BP_MasterQuest Object Reference"))
  (locals (LocalFoundQuest :type "/Game/Blueprints/Quests/BP_MasterQuest Object Reference"))
  (bind _localfoundquest (`local.LocalFoundQuest`))
  (for _array_element (`self.CurrentQuestActors`)
    (if (== (`GameplayStatics.GetObjectClass` _array_element) QuestClass)
      (set `local.LocalFoundQuest` _array_element)
      (break)))
  (`/Engine/EditorBlueprintResources/StandardMacros.IsValid` _localfoundquest
    (:`Is Valid`
      (return true _localfoundquest))
    (:`Is Not Valid`
      (return false null))))

(fn `UserConstructionScript`)